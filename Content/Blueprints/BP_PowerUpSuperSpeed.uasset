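; Super speed power-up that doubles the walk speed of the overlapping actor while active.
; OnActivated stores the actor and doubles its CharacterMovement MaxWalkSpeed; OnExpired halves it, then calls the parent's expiry logic.
; Both scale the current GetMaxSpeed result rather than restoring a saved value.
; ClientSetSpeedUp and ClientSetNormalSpeed duplicate these changes, but their calls in this graph are disconnected.
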(event `ClientSetSpeedUp`
  (bind _returnvalue (`self.GetComponentByClass` (stale `self.OnActivated` _output_get) "/Script/Engine.CharacterMovementComponent"))
  (set `CharacterMovementComponent.MaxWalkSpeed` (* (`MovementComponent.GetMaxSpeed` _returnvalue) 2.0) _returnvalue))

(event `self.OnActivated`
  (params (OverlappedActor :type "Actor Object Reference"))
  (bind _output_get (set `self.OverlappedActor` OverlappedActor))
  (`KismetSystemLibrary.PrintString` "Activated")
  (bind _returnvalue (`self.GetComponentByClass` _output_get "/Script/Engine.CharacterMovementComponent"))
  (set `CharacterMovementComponent.MaxWalkSpeed` (* (`MovementComponent.GetMaxSpeed` _returnvalue) 2.0) _returnvalue))

(event `self.OnExpired`
  (bind _returnvalue (`self.GetComponentByClass` (`self.OverlappedActor`) "/Script/Engine.CharacterMovementComponent"))
  (set `CharacterMovementComponent.MaxWalkSpeed` (/ (`MovementComponent.GetMaxSpeed` _returnvalue) 2.0) _returnvalue)
  (`parent.OnExpired`))

(event `ClientSetNormalSpeed`
  (bind _returnvalue (`self.GetComponentByClass` (`self.OverlappedActor`) "/Script/Engine.CharacterMovementComponent"))
  (set `CharacterMovementComponent.MaxWalkSpeed` (/ (`MovementComponent.GetMaxSpeed` _returnvalue) 2.0) _returnvalue))

(fn `UserConstructionScript`)