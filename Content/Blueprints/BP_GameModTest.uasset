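; Game mode test Blueprint that spawns tracker bots and awards score for kills.
; SpawnNewBot runs an EQS query in random-best-25% mode and, on success, spawns a BP_TrackerBot with a debug sphere at each returned location, skipping spots where collision adjustment fails.
; On BeginPlay it binds to OnActorKilled, which adds a fixed score to the killer's TPSPlayerState and prints the new total.
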(event `self.SpawnNewBot`
  (bind _returnvalue (`EnvQueryManager.RunEQSQuery` "/Game/Blueprints/EQS/EQS_FindSpawnLocation.EQS_FindSpawnLocation" self "RandomBest25Pct"))
  (add `EnvQueryInstanceBlueprintWrapper.OnQueryFinishedEvent` _returnvalue (delegate `OnQueryFinishedEvent_Event_0`)))

(event `OnQueryFinishedEvent_Event_0`
  (params (QueryInstance :type "EnvQueryInstanceBlueprintWrapper Object Reference") (QueryStatus :type "EEnvQueryStatus Enum" :default "Processing"))
  (switch `EEnvQueryStatus` QueryStatus
    (:`Success`
      (for _array_element (`EnvQueryInstanceBlueprintWrapper.GetResultsAsLocations` QueryInstance)
        (`KismetSystemLibrary.DrawDebugSphere` _array_element 50.0 12 (struct :`R` 1.0 :`G` 0.885502 :`A` 1.0) 5.0 2.0)
        (`|SpawnActorFromClass` "/Game/Blueprints/BP_TrackerBot.BP_TrackerBot_C" (`KismetMathLibrary.Conv_VectorToTransform` _array_element) "AdjustIfPossibleButDontSpawnIfColliding" "OverrideRootScale" null null)))))

(event `self.ReceiveBeginPlay`
  (add `self.OnActorKilled` (delegate `OnActorKilled_Event_0`)))

(event `OnActorKilled_Event_0` :!signature `self.OnActorKilled`
  (params (VictimActor :type "Actor Object Reference") (KillerActor :type "Actor Object Reference") (KillerController :type "Controller Object Reference"))
  (bind _astpsplayer_state (cast `TPSPlayerState` (`Pawn.PlayerState` (`Controller.K2_GetPawn` KillerController))))
  (`TPSPlayerState.AddScore` _astpsplayer_state 20.0)
  (`KismetSystemLibrary.PrintString` (`KismetStringLibrary.Conv_DoubleToString` (`PlayerState.Score` _astpsplayer_state)) true true (struct :`R` 0.195707 :`G` 1.0 :`A` 1.0)))

(fn `UserConstructionScript`)