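; Base Blueprint for powerup actors, handling their visual response to state changes and expiry.
; The construction script creates a dynamic material instance on the static mesh and copies its BaseColor parameter to the point light, so the glow matches the material.
; A powerup state change hides the mesh and its children while the state is true and shows them when false.
; Expiry prints a message and destroys the actor.
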(event `self.OnPowerupStateChanged`
  (params (bNewPowerupState :type Boolean))
  (`SceneComponent.SetVisibility` (`self.StaticMesh`) (not bNewPowerupState) true))

(event `self.OnExpired`
  (`KismetSystemLibrary.PrintString` "Expired")
  (`self.K2_DestroyActor`))

(fn `UserConstructionScript`
  (bind _returnvalue (`PrimitiveComponent.CreateDynamicMaterialInstance` (`self.StaticMesh`) 0 (`PrimitiveComponent.GetMaterial` (`self.StaticMesh`) 0)))
  (bind _returnvalue_2 (`MaterialInstanceDynamic.K2_GetVectorParameterValue` _returnvalue "BaseColor"))
  (`LightComponent.SetLightColor` (`self.PointLight`) _returnvalue_2 true))