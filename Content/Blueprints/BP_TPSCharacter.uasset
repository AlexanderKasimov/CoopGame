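; Third-person shooter character Blueprint that sets up the local player's HUD.
; On BeginPlay, only a locally controlled instance creates the crosshair and health indicator widgets and adds them to the viewport.
; The RestartLevel event is empty.
; A disconnected chain that would call RestartGame on the BP_CSTest game mode after a short delay never runs.
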(event `self.ReceiveBeginPlay`
  (if (`self.IsLocallyControlled`)
    (`|ExecutionSequence`
      (:`then_0`
        (bind _returnvalue (`|CreateWidget` "/Game/UI/UI_Crosshair.UI_Crosshair_C"))
        (`UserWidget.AddToViewport` _returnvalue 0))
      (:`then_1`
        (bind _returnvalue_2 (`|CreateWidget` "/Game/UI/UI_HealthIndicator.UI_HealthIndicator_C"))
        (`UserWidget.AddToViewport` _returnvalue_2 0)))))

(event `self.RestartLevel`)

(fn `UserConstructionScript`)