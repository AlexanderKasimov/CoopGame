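; BP_AdvancedAI is an AI combatant that arms itself and starts its behavior tree when play begins.
; On BeginPlay it randomly spawns either an AI grenade launcher or an AI rifle, runs BT_AdvancedAI on its controller, and clears the isHealing blackboard flag.
; A node that would set the player pawn as TargetActor exists but is disconnected, so this graph never assigns a target.
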(event `self.ReceiveBeginPlay`
  (`self.SpawnWeapon` (select `bool` (`KismetMathLibrary.RandomBool`) :`false` "/Game/Blueprints/BP_Rifle_AI.BP_Rifle_AI_C" :`true` "/Game/Blueprints/BP_GrenadeLauncher_AI.BP_GrenadeLauncher_AI_C" :!type "TPSBaseWeapon Class Reference"))
  (`AIController.RunBehaviorTree` (`AIBlueprintHelperLibrary.GetAIController` self) "/Game/AI/BT_AdvancedAI.BT_AdvancedAI")
  (`BlackboardComponent.SetValueAsBool` (`AIBlueprintHelperLibrary.GetBlackboard` self) "isHealing" false))

(fn `UserConstructionScript`)