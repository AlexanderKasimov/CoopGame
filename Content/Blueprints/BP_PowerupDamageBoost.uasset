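; BP_PowerupDamageBoost is a timed powerup that boosts the current weapon of every BP_TPSCharacter in the level.
; On activation it loops over all those characters, doubles each current weapon's BaseDamage and adds a fixed amount of ammo.
; On expiry it halves the damage of whichever weapon each character then holds, keeps the added ammo, and calls the parent OnExpired.
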(event `self.OnActivated`
  (params (OverlappedActor :type "Actor Object Reference"))
  (bind _outactors (`GameplayStatics.GetAllActorsOfClass` "/Game/Blueprints/BP_TPSCharacter.BP_TPSCharacter_C"))
  (for _array_element _outactors
    (bind _returnvalue (`TPSCharacter.GetCurrentWeapon` _array_element))
    (set `TPSBaseWeapon.BaseDamage` (* (`TPSBaseWeapon.BaseDamage` _returnvalue) 2.0) _returnvalue)
    (set `TPSBaseWeapon.CurrentAmmo` (+ (`TPSBaseWeapon.CurrentAmmo` _returnvalue) 135.0) _returnvalue)))

(event `self.OnExpired`
  (bind _outactors (`GameplayStatics.GetAllActorsOfClass` "/Game/Blueprints/BP_TPSCharacter.BP_TPSCharacter_C"))
  (for _array_element _outactors
    (bind _returnvalue (`TPSCharacter.GetCurrentWeapon` _array_element))
    (set `TPSBaseWeapon.BaseDamage` (/ (`TPSBaseWeapon.BaseDamage` _returnvalue) 2.0) _returnvalue))
  (`parent.OnExpired`))

(fn `UserConstructionScript`
  (`parent.UserConstructionScript`))